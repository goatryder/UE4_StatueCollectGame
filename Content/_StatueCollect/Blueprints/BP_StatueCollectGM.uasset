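; Game mode for a statue collection game where the player races a countdown to score points and advance stages.
; A registered statue manager starts the match and reports pickups, which award stage-scaled points, and level-ups, which add extra time.
; Tick drains the countdown and at zero ends the match once, then restarts the game after a delay.
; Dispatchers broadcast score, stage, timer and game-over changes.
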(event `self.ReceiveBeginPlay`
  (set `self.Countdown` (`self.InitialCountdown`)))

(event `AddScore`
  (params (Value :type Integer))
  (set `self.Score` (+ (`self.Score`) Value))
  (`self.ScoreChanged` (`self.Score`)))

(event `InitStatueManager`
  (params (StatueManager :type "/Game/_StatueCollect/Blueprints/BP_StatueManager Object Reference"))
  (bind _output_get (set `self.StatueManager` StatueManager))
  (add `/Game/_StatueCollect/Blueprints/BP_StatueManager.StatueCollected` _output_get (delegate `OnStatueCollected`))
  (add `/Game/_StatueCollect/Blueprints/BP_StatueManager.StageLevelUp` _output_get (delegate `OnStageLevelUp`))
  (`self.StartMatch`))

(event `OnStatueCollected`
  (params (CollectedTotal :type Integer) (StageLevel :type Integer))
  (`self.AddScore` (* StageLevel (`self.StatueScoreBase`))))

(event `OnStageLevelUp`
  (params (Old :type Integer) (New :type Integer))
  (set `self.Countdown` (+ (`self.Countdown`) (`self.StageLevelUpExtraTime`)))
  (bind _output_get (set `self.Stage` New))
  (`self.StageChanged` _output_get))

(event `HandleLooseCondition`
  (if (not (`self.bIsLoosed`))
    (set `self.bIsLoosed` true)
    (`self.EndMatch`)
    (`self.GameOverObserver` (`self.OnLooseRestartTime`))
    (`self.RestartLevel`)))

(event `RestartLevel`
  (`KismetSystemLibrary.Delay` (`self.OnLooseRestartTime`))
  (`self.RestartGame`))

(event `self.ReceiveTick`
  (params (DeltaSeconds :type "Float (single-precision)"))
  (bind _returnvalue (- (`self.Countdown`) DeltaSeconds))
  (`|ExecutionSequence`
    (:`then_0`
      ;[1 1 1] Countdown
      (if (< _returnvalue 0.0)
        (set `self.Countdown` 0.0)
        (`self.HandleLooseCondition`)
        (else
          (set `self.Countdown` _returnvalue))))
    (:`then_1`
      (`self.TimerUpdated` (`self.Countdown`)))))

(fn `UserConstructionScript`)