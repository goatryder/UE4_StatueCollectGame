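; HUD for the Statue Collect game mode that shows stage, timer, score and a game-over restart countdown.
; On BeginPlay it creates the StatueCollect and GameOver widgets, keeping GameOver hidden, and caches the BP_StatueCollectGM reference.
; It binds to the game mode's stage, timer, score and game-over events, forwarding each value to the matching widget.
; Game over reveals the GameOver widget and starts its countdown with the restart time.
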(event `self.ReceiveBeginPlay`
  (bind _statuecollectgm (`self.StatueCollectGM`))
  (`|ExecutionSequence`
    (:`then_0`
      ;[1 1 1] Statue Collect Widget
      (bind _returnvalue (`|CreateWidget` "/Game/_StatueCollect/UI/WBP_StatueCollect.WBP_StatueCollect_C"))
      (bind _output_get (set `self.StatueCollectWidget` _returnvalue))
      (`UserWidget.AddToViewport` _output_get 0)
      (bind _returnvalue_2 (`|CreateWidget` "/Game/_StatueCollect/UI/WBP_GameOver.WBP_GameOver_C"))
      (bind _output_get_2 (set `self.GameOverWidget` _returnvalue_2))
      (`Widget.SetVisibility` _output_get_2 "Hidden")
      (`UserWidget.AddToViewport` _output_get_2 0)
      ;[1 1 1] StatueColect GM ref
      (bind _asbp_statue_collect_gm (cast `/Game/_StatueCollect/Blueprints/BP_StatueCollectGM` (`GameplayStatics.GetGameMode`)))
      (set `self.StatueCollectGM` _asbp_statue_collect_gm))
    (:`then_1`
      ;[1 1 1] Bind GM Events to Change Widget
      (`/Engine/EditorBlueprintResources/StandardMacros.IsValid` _statuecollectgm
        (:`Is Valid`
          (add `/Game/_StatueCollect/Blueprints/BP_StatueCollectGM.StageChanged` _statuecollectgm (delegate `OnStageChanged`))
          (add `/Game/_StatueCollect/Blueprints/BP_StatueCollectGM.TimerUpdated` _statuecollectgm (delegate `OnTimerUpdated`))
          (add `/Game/_StatueCollect/Blueprints/BP_StatueCollectGM.ScoreChanged` _statuecollectgm (delegate `OnScoreChanged`))
          (add `/Game/_StatueCollect/Blueprints/BP_StatueCollectGM.GameOverObserver` _statuecollectgm (delegate `OnGameOver`)))))))

(event `OnStageChanged`
  (params (NewStage :type Integer))
  (bind _statuecollectwidget (`self.StatueCollectWidget`))
  ;[1 1 1] Bind GM Events to Change Widget
  (`/Engine/EditorBlueprintResources/StandardMacros.IsValid` _statuecollectwidget
    (:`Is Valid`
      (`/Game/_StatueCollect/UI/WBP_StatueCollect.UpdateStageCount` _statuecollectwidget NewStage))))

(event `OnTimerUpdated`
  (params (Countdown :type "Float (double-precision)"))
  (bind _statuecollectwidget (`self.StatueCollectWidget`))
  ;[1 1 1] Bind GM Events to Change Widget
  (`/Engine/EditorBlueprintResources/StandardMacros.IsValid` _statuecollectwidget
    (:`Is Valid`
      (`/Game/_StatueCollect/UI/WBP_StatueCollect.UpdateTimeCount` _statuecollectwidget Countdown))))

(event `OnScoreChanged`
  (params (NewScore :type Integer))
  (bind _statuecollectwidget (`self.StatueCollectWidget`))
  ;[1 1 1] Bind GM Events to Change Widget
  (`/Engine/EditorBlueprintResources/StandardMacros.IsValid` _statuecollectwidget
    (:`Is Valid`
      (`/Game/_StatueCollect/UI/WBP_StatueCollect.UpdateScoreCount` _statuecollectwidget NewScore))))

(event `OnGameOver`
  (params (RestartTime :type "Float (double-precision)"))
  (bind _gameoverwidget (`self.GameOverWidget`))
  ;[1 1 1] Bind GM Events to Change Widget
  (`/Engine/EditorBlueprintResources/StandardMacros.IsValid` _gameoverwidget
    (:`Is Valid`
      (`Widget.SetVisibility` _gameoverwidget "Visible")
      (`/Game/_StatueCollect/UI/WBP_GameOver.StartCountdown` _gameoverwidget RestartTime))))

(fn `UserConstructionScript`)