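; Collectible statue that reports itself to BP_StatueManager on spawn and again when the player overlaps its sphere.
; A Tick timer, shortened as the manager's stage rises, plays a sound and after a short delay asks the manager to relocate it.
; Between moves, its point light dims as the timer runs out and it yaws to face the player using dot and cross products.
; It starts in one of three random dance poses.
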(event `self.ReceiveBeginPlay`
  (`|ExecutionSequence`
    (:`then_0`
      (`SkeletalMeshComponent.SetAnimation` (`self.SkeletalMesh`) (select `int` (`KismetMathLibrary.RandomIntegerInRange` 0 2) :`0` "/Game/_StatueCollect/MixamoAnims/AnimsRetargetedToUE/DancePos1.DancePos1" :`1` "/Game/_StatueCollect/MixamoAnims/AnimsRetargetedToUE/DancePos2.DancePos2" :`2` "/Game/_StatueCollect/MixamoAnims/AnimsRetargetedToUE/DancePos3.DancePos3" :!type "AnimationAsset Object Reference")))
    (:`then_1`
      (`/Engine/EditorBlueprintResources/StandardMacros.IsValid` (`self.StatueManager`)
        (:`Is Valid`
          (`/Game/_StatueCollect/Blueprints/BP_StatueManager.OnStatueSpawned` (`self.StatueManager`) self)
          ;[1 1 1] Update Pos Change Timer
          (`self.SetTimeToChangePos` (`/Game/_StatueCollect/Blueprints/BP_StatueManager.Stage` (`self.StatueManager`)))
          (add `/Game/_StatueCollect/Blueprints/BP_StatueManager.StageLevelUp` (`self.StatueManager`) (delegate `OnStageLevelChange_UpdateChangePosTime`)))))))

(event `OnStageLevelChange_UpdateChangePosTime`
  (params (Old :type Integer) (New :type Integer))
  ;[1 1 1] Update Pos Change Timer
  (`self.SetTimeToChangePos` New))

(event `SetTimeToChangePos`
  (params (Stage :type Integer))
  ;[1 1 1] Update Pos Change Timer
  (set `self.TimeToChangePos` (- (`self.TimeDecreaseByStage`) (`KismetMathLibrary.Conv_IntToDouble` Stage))))

(event `self.Sphere.OnComponentBeginOverlap`
  (params (OverlappedComponent :type "PrimitiveComponent Object Reference") (OtherActor :type "Actor Object Reference") (OtherComp :type "PrimitiveComponent Object Reference") (OtherBodyIndex :type Integer) (bFromSweep :type Boolean) (SweepResult :type "HitResult Structure (by ref)"))
  (`/Engine/EditorBlueprintResources/StandardMacros.IsValid` (`self.StatueManager`)
    (:`Is Valid`
      (if (== OtherActor (`/Game/_StatueCollect/Blueprints/BP_StatueManager.PlayerCharacter` (`self.StatueManager`)))
        (`/Game/_StatueCollect/Blueprints/BP_StatueManager.OnStatueCollected` (`self.StatueManager`) self)))))

(event `self.ReceiveTick`
  (params (DeltaSeconds :type "Float (single-precision)"))
  (bind _statuemanager (`self.StatueManager`))
  (set `self.TimeSincePosChange` (+ (`self.TimeSincePosChange`) DeltaSeconds))
  (if (>= (`self.TimeSincePosChange`) (`self.TimeToChangePos`))
    (set `self.TimeSincePosChange` 0.0)
    (`AudioComponent.Play` (`self.AudioMoved`) 0.0)
    (`KismetSystemLibrary.Delay` (`self.TimeChangePosSoundOffset`))
    (`/Engine/EditorBlueprintResources/StandardMacros.IsValid` _statuemanager
      (:`Is Valid`
        (`/Game/_StatueCollect/Blueprints/BP_StatueManager.ChangeStatuePosition` _statuemanager self)))
    (else
      ;[1 1 1] fx
      (`self.PointLightChangeIntensity`)
      (`self.FindYawToCharacter`))))

(event `PointLightChangeIntensity`
  (`LightComponent.SetIntensity` (`self.PointLight`) (`KismetMathLibrary.MapRangeClamped` (/ (`self.TimeSincePosChange`) (`self.TimeToChangePos`)) 0.0 1.0 10000.0 1000.0)))

(fn `FindYawToCharacter`
  (bind _returnvalue (`self.GetActorForwardVector`))
  (bind (_returnvalue_roll _returnvalue_pitch _returnvalue_yaw) (`KismetMathLibrary.BreakRotator` (`self.K2_GetActorRotation`)))
  (bind (_returnvalue_x _returnvalue_y) (`KismetMathLibrary.BreakVector` (`self.K2_GetActorLocation`)))
  (bind _statuemanager (`self.StatueManager`))
  (bind _playercharacter (`/Game/_StatueCollect/Blueprints/BP_StatueManager.PlayerCharacter` _statuemanager))
  (bind (_returnvalue_x_2 _returnvalue_y_2) (`KismetMathLibrary.BreakVector` (`self.K2_GetActorLocation` _playercharacter)))
  (bind _returnvalue_2 (`KismetMathLibrary.Normal` (- (`KismetMathLibrary.MakeVector` _returnvalue_x_2 _returnvalue_y_2) (`KismetMathLibrary.MakeVector` _returnvalue_x _returnvalue_y))))
  (`/Engine/EditorBlueprintResources/StandardMacros.IsValid` _statuemanager
    (:`Is Valid`
      (`/Engine/EditorBlueprintResources/StandardMacros.IsValid` _playercharacter
        (:`Is Valid`
          (`|ExecutionSequence`
            (:`then_1`
              (`self.K2_SetActorRotation` (`KismetMathLibrary.MakeRotator` 0.0 0.0 (+ _returnvalue_yaw (* (`KismetMathLibrary.DegAcos` (`KismetMathLibrary.Dot_VectorVector` _returnvalue _returnvalue_2)) (`KismetMathLibrary.SignOfFloat` (`KismetMathLibrary.Dot_VectorVector` (`KismetMathLibrary.Cross_VectorVector` _returnvalue _returnvalue_2) (0.0 0.0 1.0))))))))))))))

(fn `UserConstructionScript`
  ;[1 1 1] If placed from editor
  (bind _returnvalue (`GameplayStatics.GetActorOfClass` "/Game/_StatueCollect/Blueprints/BP_StatueManager.BP_StatueManager_C"))
  (set `self.StatueManager` _returnvalue))