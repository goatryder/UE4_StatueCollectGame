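; Manager actor for the statue-collecting game that keeps the level stocked with statues and tracks collection progress, registering itself with BP_StatueCollectGM.
; Spawning and repositioning use EQS_SelectSpawnPoint with random best-25% results, and each successful spawn retries until the statue cap is reached.
; Collecting destroys the statue, broadcasts totals and advances the stage at set intervals up to a maximum.
; Collection also triggers replacement spawns, except when the stage increases.
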(event `self.ReceiveBeginPlay`
  ;[1 1 1] Initialization
  (`|ExecutionSequence`
    (:`then_0`
      ;;[1 1 1] Hack To get Player reference
      (bind _returnvalue (`GameplayStatics.GetActorOfClass` "/Game/ThirdPersonBP/Blueprints/ThirdPersonCharacter.ThirdPersonCharacter_C"))
      (set `self.PlayerCharacter` _returnvalue))
    (:`then_1`
      (`KismetSystemLibrary.Delay` 0.2)
      ;;[1 1 1] Count already placed statues
      (bind _outactors (`GameplayStatics.GetAllActorsOfClass` "/Game/_StatueCollect/Blueprints/BP_Statue.BP_Statue_C"))
      (set `self.StatueNum` (`KismetArrayLibrary.Array_Length` _outactors))
      (`self.TrySpawnNewStatue`))
    (:`then_2`
      (bind _asbp_statue_collect_gm (cast `/Game/_StatueCollect/Blueprints/BP_StatueCollectGM` (`GameplayStatics.GetGameMode`)))
      (bind _output_get (set `self.GameMode` _asbp_statue_collect_gm))
      (`/Game/_StatueCollect/Blueprints/BP_StatueCollectGM.InitStatueManager` _output_get self))))

(event `OnStatueCollected`
  (params (Statue :type "/Game/_StatueCollect/Blueprints/BP_Statue Object Reference"))
  (bind _stage (`self.Stage`))
  (bind _totalstatuecollected (`self.TotalStatueCollected`))
  ;[1 1 1] On Sstatue Collected
  (`|ExecutionSequence`
    (:`then_0`
      (`self.K2_DestroyActor` Statue)
      (`/Engine/EditorBlueprintResources/StandardMacros.DecrementInt` (`self.StatueNum`)
        (:`  `
          ;;[1 1 1] Update Total
          (`/Engine/EditorBlueprintResources/StandardMacros.IncrementInt` _totalstatuecollected
            (:`  `
              (`KismetSystemLibrary.PrintString` (`KismetStringLibrary.Concat_StrStr` "Total Statue Collected " (`KismetStringLibrary.Conv_IntToString` _totalstatuecollected)))
              ;;[1 1 1] Stage Level Up
              (if (== (mod (`self.TotalStatueCollected`) (`self.StatueCollectToLevelUp`)) 0)
                (if (!= (`self.Stage`) (`self.StageMax`))
                  (bind _result (`/Engine/EditorBlueprintResources/StandardMacros.IncrementInt` (`self.Stage`))
                    (:`  `
                      (`self.StageLevelUp` (- _result 1) _result)
                      (`KismetSystemLibrary.PrintString` (`KismetStringLibrary.Concat_StrStr` "New Stage: " (`KismetStringLibrary.Conv_IntToString` _result)))))
                  (else
                    (`self.StageLevelUp` _stage _stage)
                    (`self.TrySpawnNewStatue` :!label _label)))
                (else
                  (goto _label))))))))
    (:`then_1`
      (`self.StatueCollected` (`self.TotalStatueCollected`) (`self.Stage`)))))

(event `OnStatueSpawned`
  (params (Statue :type "/Game/_StatueCollect/Blueprints/BP_Statue Object Reference"))
  ;[1 1 1] On Statue Spawned
  (`/Engine/EditorBlueprintResources/StandardMacros.IncrementInt` (`self.StatueNum`)))

(event `ChangeStatuePosition`
  (params (Statue :type "/Game/_StatueCollect/Blueprints/BP_Statue Object Reference"))
  ;[1 1 1] Change Statue Pos
  (bind _returnvalue (`EnvQueryManager.RunEQSQuery` "/Game/_StatueCollect/Blueprints/EQS_SelectSpawnPoint.EQS_SelectSpawnPoint" self "RandomBest25Pct"))
  (add `EnvQueryInstanceBlueprintWrapper.OnQueryFinishedEvent` _returnvalue (delegate `OnQueryFinished_ChangeStatueLocation`)))

(event `OnQueryFinished_ChangeStatueLocation`
  (params (QueryInstance :type "EnvQueryInstanceBlueprintWrapper Object Reference") (QueryStatus :type "EEnvQueryStatus Enum" :default "Processing"))
  ;[1 1 1] Change Statue Pos
  (switch `EEnvQueryStatus` QueryStatus
    (:`Success`
      (bind _resultlocations (`EnvQueryInstanceBlueprintWrapper.GetQueryResultsAsLocations` QueryInstance))
      (`self.K2_SetActorLocation` (stale `ChangeStatuePosition` Statue) (`|GetArrayItem` _resultlocations) false false))))

(event `TrySpawnNewStatue`
  ;[1 1 1] Spawn Statue
  (if (< (`self.StatueNum`) (`self.StatueNumMax`))
    (bind _returnvalue (`EnvQueryManager.RunEQSQuery` "/Game/_StatueCollect/Blueprints/EQS_SelectSpawnPoint.EQS_SelectSpawnPoint" self "RandomBest25Pct"))
    (add `EnvQueryInstanceBlueprintWrapper.OnQueryFinishedEvent` _returnvalue (delegate `OnQueryFinished_SpawnStatue`))))

(event `OnQueryFinished_SpawnStatue`
  (params (QueryInstance :type "EnvQueryInstanceBlueprintWrapper Object Reference") (QueryStatus :type "EEnvQueryStatus Enum" :default "Processing"))
  ;[1 1 1] Spawn Statue
  (switch `EEnvQueryStatus` QueryStatus
    (:`Success`
      (bind _resultlocations (`EnvQueryInstanceBlueprintWrapper.GetQueryResultsAsLocations` QueryInstance))
      (`|SpawnActorFromClass` (`self.StatueClass`) (`KismetMathLibrary.MakeTransform` (`|GetArrayItem` _resultlocations)) "AdjustIfPossibleButAlwaysSpawn" "OverrideRootScale" null self null)
      ;;[1 1 1] Recursive loop
      (`self.TrySpawnNewStatue`))))

(fn `UserConstructionScript`)